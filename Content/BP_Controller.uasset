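; Player controller that turns input into pawn movement and character interaction.
; Forward and right axes move the controlled pawn along fixed world directions, independent of pawn or camera rotation.
; The Interaction action casts the pawn to BP_Character and calls its OnInteract.
; A mouse movement toggle still sets AddMovement, but the logic that moves the pawn toward the cursor is disconnected and never runs.
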(event `InputAction|Toggle Movement`
  (params (Key :type "Key Structure"))
  ;[1 1 1] Movement Mouse
  (:`Pressed`
    (set `self.AddMovement` true))
  (:`Released`
    (set `self.AddMovement` false)))

(event `self.ReceiveTick`
  (params (DeltaSeconds :type "Float (single-precision)"))
  ;[1 1 1] Movement Mouse
)

(event `InputAxis|Movement Forward`
  (params (AxisValue :type "Float (single-precision)"))
  ;[1 1 1] Movement Keys
  (`Pawn.AddMovementInput` (`self.K2_GetPawn`) (`KismetMathLibrary.GetForwardVector` (struct)) AxisValue false))

(event `InputAxis|Movement Right`
  (params (AxisValue :type "Float (single-precision)"))
  ;[1 1 1] Movement Keys
  (`Pawn.AddMovementInput` (`self.K2_GetPawn`) (`KismetMathLibrary.GreaterGreater_VectorRotator` (`KismetMathLibrary.GetForwardVector` (struct)) (struct :`Yaw` 90.0)) AxisValue false))

(event `InputAction|Interaction`
  (params (Key :type "Key Structure"))
  (:`Pressed`
    (bind _asbp_character (cast `/Game/BP_Character` (`self.K2_GetPawn`)))
    (`/Game/BP_Character.On Interact` _asbp_character)))

(fn `UserConstructionScript`)